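; AI controller Blueprint that drives a pawn representing the player through a behavior tree.
; StartRepresentation runs PlayerRepresentationBT, and events write target location, look location and sitting state into its blackboard.
; StopRepresentation hands the pawn to the ScrollingPlayerController's StopAI, and SyncRotation copies this controller's control rotation onto that player controller.
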(event Custom|StartRepresentation
  (AI|RunBehaviorTree "/Game/Blueprints/AI/PlayerRepresentationBT.PlayerRepresentationBT"))

(event Custom|SetTargetLoc
  (params (TargetLoc :type Vector))
  (AI|Components|Blackboard|SetValueasVector (AI|GetBlackboard 0) (Utilities|Name|MakeLiteralName "TargetLoc") TargetLoc))

(event Custom|Sit
  (AI|Components|Blackboard|SetValueasBool (AI|GetBlackboard 0) (Utilities|Name|MakeLiteralName "Sitting") true))

(event Custom|Stand
  (AI|Components|Blackboard|SetValueasBool (AI|GetBlackboard 0) (Utilities|Name|MakeLiteralName "Sitting") false))

(event Custom|SyncRotation
  (Pawn|SetControlRotation (Variables|Default|GetScrollingPlayerController) (Pawn|GetControlRotation :!class /Script/Engine.Controller)))

(event Custom|SetLookLoc
  (params (LookLoc :type Vector))
  (AI|Components|Blackboard|SetValueasVector (AI|GetBlackboard 0) (Utilities|Name|MakeLiteralName "LookLoc") LookLoc))

(event Custom|StopRepresentation
  (params (InPawn :type Pawn%20Object%20Reference))
  (Default|StopAI (Variables|Default|GetScrollingPlayerController) InPawn))

(event EventBeginPlay)

(fn ConstructionScript)