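; Editor-placed controller that applies shared point and spot light settings to a group of BP_Overheadlight_01 fixtures, apparently coach lighting.
; Its construction script gathers every fixture whose IsCouch check matches ControlGroup, then pushes light settings, Cycle and AutoFlash and resets each one.
; Reset reapplies settings except AutoFlash; UpdateLightParameters writes to the components directly, for all gathered lights or one coach number.
; BeginPlay and Tick are empty, so the event graph drives nothing at runtime.
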(event EventBeginPlay)

(event Collision|EventActorBeginOverlap
  (params (OtherActor :type Actor%20Object%20Reference)))

(event EventTick
  (params (DeltaSeconds :type Float%20%28single-precision%29)))

(fn ConstructionScript
  (Utilities|Array|Clear (Variables|Default|GetLights))
  (bind _outactors (Actor|GetAllActorsOfClass "/Game/SubwayTrain/Blueprints/BP_Overheadlight_01.BP_Overheadlight_01_C"))
  (for _array_element _outactors
    (bind _newparam (Default|IsCouch _array_element (Variables|Default|GetControlGroup)))
    (if _newparam
      (Utilities|Array|Add (Variables|Default|GetLights) _array_element)))
  (for _array_element_2 (Variables|Default|GetLights)
    (Utilities|FlowControl|Sequence
      (:then_0
        (Default|ChangePointsSetting _array_element_2 (Variables|PointLight|GetPoints_Intensity) (Variables|PointLight|GetPoints_Color) (Variables|PointLight|GetPoints_Attenuation) (Variables|PointLight|GetPoints_SoftR) (Variables|PointLight|GetPoint_on/off) (Variables|PointLight|GetPoints_Temperature)))
      (:then_1
        (Default|ChangeSpotsSetting _array_element_2 (Variables|Spot_Light|GetSpots_Brightness) (Variables|Spot_Light|GetSpot%20Color) (Variables|Spot_Light|GetSpot%20Attenuation) (Variables|Spot_Light|GetSpot%20Soft%20R) (Variables|Spot_Light|GetSpot_on/off) (Variables|Spot_Light|GetSpot%20Temperature)))
      (:then_2
        (Variables|/Game/SubwayTrain/Blueprints/BP_Overheadlight_01.BP_Overheadlight_01_C|SetCycle _array_element_2 (Variables|Default|GetCycle))
        (Default|Reset _array_element_2)
        (Variables|/Game/SubwayTrain/Blueprints/BP_Overheadlight_01.BP_Overheadlight_01_C|SetAutoFlash _array_element_2 (Variables|Default|GetAutoFlash))))))

(fn UpdateLightParameters
  (params (CoachNum :type Float%20%28double-precision%29))
  (if (== CoachNum 0.0)
    (for _array_element (Variables|Default|GetLights)
      (Rendering|Components|Light|SetIntensity (Variables|/Game/SubwayTrain/Blueprints/BP_Overheadlight_01.BP_Overheadlight_01_C|GetPointLight _array_element) (Variables|PointLight|GetPoints_Intensity))
      (Rendering|Components|Light|SetLightColor (Variables|/Game/SubwayTrain/Blueprints/BP_Overheadlight_01.BP_Overheadlight_01_C|GetPointLight _array_element) (Variables|PointLight|GetPoints_Color) true)
      (Rendering|Lighting|SetAttenuationRadius (Variables|/Game/SubwayTrain/Blueprints/BP_Overheadlight_01.BP_Overheadlight_01_C|GetPointLight _array_element) (Variables|PointLight|GetPoints_Attenuation))
      (Class|PointLightComponent|SetSoftSourceRadius (Variables|/Game/SubwayTrain/Blueprints/BP_Overheadlight_01.BP_Overheadlight_01_C|GetPointLight _array_element) (Variables|PointLight|GetPoints_SoftR))
      (Rendering|SetVisibility (Variables|/Game/SubwayTrain/Blueprints/BP_Overheadlight_01.BP_Overheadlight_01_C|GetPointLight _array_element) (Variables|PointLight|GetPoint_on/off) false)
      (Class|LightComponent|SetTemperature (Variables|/Game/SubwayTrain/Blueprints/BP_Overheadlight_01.BP_Overheadlight_01_C|GetPointLight _array_element) (Variables|PointLight|GetPoints_Temperature))
      (Rendering|Components|Light|SetIntensity (Variables|/Game/SubwayTrain/Blueprints/BP_Overheadlight_01.BP_Overheadlight_01_C|GetSpotLight _array_element) (Variables|Spot_Light|GetSpots_Brightness))
      (Rendering|Components|Light|SetLightColor (Variables|/Game/SubwayTrain/Blueprints/BP_Overheadlight_01.BP_Overheadlight_01_C|GetSpotLight _array_element) (Variables|Spot_Light|GetSpot%20Color) true)
      (Rendering|Lighting|SetAttenuationRadius (Variables|/Game/SubwayTrain/Blueprints/BP_Overheadlight_01.BP_Overheadlight_01_C|GetSpotLight _array_element) (Variables|Spot_Light|GetSpot%20Attenuation))
      (Class|PointLightComponent|SetSoftSourceRadius (Variables|/Game/SubwayTrain/Blueprints/BP_Overheadlight_01.BP_Overheadlight_01_C|GetSpotLight _array_element) (Variables|Spot_Light|GetSpot%20Soft%20R))
      (Rendering|SetVisibility (Variables|/Game/SubwayTrain/Blueprints/BP_Overheadlight_01.BP_Overheadlight_01_C|GetSpotLight _array_element) (Variables|Spot_Light|GetSpot_on/off) false)
      (Class|LightComponent|SetTemperature (Variables|/Game/SubwayTrain/Blueprints/BP_Overheadlight_01.BP_Overheadlight_01_C|GetSpotLight _array_element) (Variables|Spot_Light|GetSpot%20Temperature))
      (Variables|/Game/SubwayTrain/Blueprints/BP_Overheadlight_01.BP_Overheadlight_01_C|SetCycle _array_element (Variables|Default|GetCycle)))
    (else
      (for _array_element_2 (Variables|Default|GetLights)
        (bind _coachnum (Default|GetCoachNumber _array_element_2))
        (if (== _coachnum CoachNum)
          (Rendering|Components|Light|SetIntensity (Variables|/Game/SubwayTrain/Blueprints/BP_Overheadlight_01.BP_Overheadlight_01_C|GetPointLight _array_element_2) (Variables|PointLight|GetPoints_Intensity))
          (Rendering|Components|Light|SetLightColor (Variables|/Game/SubwayTrain/Blueprints/BP_Overheadlight_01.BP_Overheadlight_01_C|GetPointLight _array_element_2) (Variables|PointLight|GetPoints_Color) true)
          (Rendering|Lighting|SetAttenuationRadius (Variables|/Game/SubwayTrain/Blueprints/BP_Overheadlight_01.BP_Overheadlight_01_C|GetPointLight _array_element_2) (Variables|PointLight|GetPoints_Attenuation))
          (Class|PointLightComponent|SetSoftSourceRadius (Variables|/Game/SubwayTrain/Blueprints/BP_Overheadlight_01.BP_Overheadlight_01_C|GetPointLight _array_element_2) (Variables|PointLight|GetPoints_SoftR))
          (Rendering|SetVisibility (Variables|/Game/SubwayTrain/Blueprints/BP_Overheadlight_01.BP_Overheadlight_01_C|GetPointLight _array_element_2) (Variables|PointLight|GetPoint_on/off) false)
          (Class|LightComponent|SetTemperature (Variables|/Game/SubwayTrain/Blueprints/BP_Overheadlight_01.BP_Overheadlight_01_C|GetPointLight _array_element_2) (Variables|PointLight|GetPoints_Temperature))
          (Rendering|Components|Light|SetIntensity (Variables|/Game/SubwayTrain/Blueprints/BP_Overheadlight_01.BP_Overheadlight_01_C|GetSpotLight _array_element_2) (Variables|Spot_Light|GetSpots_Brightness))
          (Rendering|Components|Light|SetLightColor (Variables|/Game/SubwayTrain/Blueprints/BP_Overheadlight_01.BP_Overheadlight_01_C|GetSpotLight _array_element_2) (Variables|Spot_Light|GetSpot%20Color) true)
          (Rendering|Lighting|SetAttenuationRadius (Variables|/Game/SubwayTrain/Blueprints/BP_Overheadlight_01.BP_Overheadlight_01_C|GetSpotLight _array_element_2) (Variables|Spot_Light|GetSpot%20Attenuation))
          (Class|PointLightComponent|SetSoftSourceRadius (Variables|/Game/SubwayTrain/Blueprints/BP_Overheadlight_01.BP_Overheadlight_01_C|GetSpotLight _array_element_2) (Variables|Spot_Light|GetSpot%20Soft%20R))
          (Rendering|SetVisibility (Variables|/Game/SubwayTrain/Blueprints/BP_Overheadlight_01.BP_Overheadlight_01_C|GetSpotLight _array_element_2) (Variables|Spot_Light|GetSpot_on/off) false)
          (Class|LightComponent|SetTemperature (Variables|/Game/SubwayTrain/Blueprints/BP_Overheadlight_01.BP_Overheadlight_01_C|GetSpotLight _array_element_2) (Variables|Spot_Light|GetSpot%20Temperature))
          (Variables|/Game/SubwayTrain/Blueprints/BP_Overheadlight_01.BP_Overheadlight_01_C|SetCycle _array_element_2 (Variables|Default|GetCycle)))))))

(fn Reset
  (for _array_element (Variables|Default|GetLights)
    (Utilities|FlowControl|Sequence
      (:then_0
        (Default|ChangePointsSetting _array_element (Variables|PointLight|GetPoints_Intensity) (Variables|PointLight|GetPoints_Color) (Variables|PointLight|GetPoints_Attenuation) (Variables|PointLight|GetPoints_SoftR) (Variables|PointLight|GetPoint_on/off) (Variables|PointLight|GetPoints_Temperature)))
      (:then_1
        (Default|ChangeSpotsSetting _array_element (Variables|Spot_Light|GetSpots_Brightness) (Variables|Spot_Light|GetSpot%20Color) (Variables|Spot_Light|GetSpot%20Attenuation) (Variables|Spot_Light|GetSpot%20Soft%20R) (Variables|Spot_Light|GetSpot_on/off) (Variables|Spot_Light|GetSpot%20Temperature)))
      (:then_2
        (Variables|/Game/SubwayTrain/Blueprints/BP_Overheadlight_01.BP_Overheadlight_01_C|SetCycle _array_element (Variables|Default|GetCycle))
        (Default|Reset _array_element)))))