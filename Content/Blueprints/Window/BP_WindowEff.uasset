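; BP_WindowEff is a window effect that reveals ten decals one after another, apparently hands judging by the event names.
; BeginPlay hides the decals and stores them in an ordered array.
; StartShowHand resets the index and starts ShowHand, which re-calls itself after each Delay and reveal until the array ends.
; Each delay is the difference of successive base-10 logarithms, so the decals appear at an accelerating pace.
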(event Custom|StartShowHand
  (Variables|Default|SetIdx 0)
  (CallFunction|ShowHand))

(event Custom|ShowHand
  (bind _decalarray (Variables|Default|GetDecalArray))
  (if (Utilities|Array|IsValidIndex _decalarray (Variables|Default|GetIdx))
    (Utilities|FlowControl|Delay (- (Math|Float|Log (Math|Conversions|ToFloat(Integer) (+ (Variables|Default|GetIdx) 2)) 1e+01) (Math|Float|Log (Math|Conversions|ToFloat(Integer) (+ (Variables|Default|GetIdx) 1)) 1e+01)))
    (Rendering|SetVisibility (Utilities|Array|Get(acopy) _decalarray (Variables|Default|GetIdx)) true false)
    (Variables|Default|SetIdx (+ (Variables|Default|GetIdx) 1))
    (CallFunction|ShowHand)))

(event EventBeginPlay
  (bind _decal1 (Variables|Default|GetDecal1))
  (Rendering|SetVisibility _decal1 false false)
  (Variables|Default|SetDecalArray (Utilities|Array|MakeArray _decal1 (Variables|Default|GetDecal2) (Variables|Default|GetDecal3) (Variables|Default|GetDecal4) (Variables|Default|GetDecal5) (Variables|Default|GetDecal6) (Variables|Default|GetDecal7) (Variables|Default|GetDecal8) (Variables|Default|GetDecal9) (Variables|Default|GetDecal))))

(fn ConstructionScript)