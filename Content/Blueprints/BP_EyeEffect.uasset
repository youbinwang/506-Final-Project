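; BP_EyeEffect is a post-process Blueprint that simulates eyes blinking, opening and closing as a screen effect.
; The construction script creates a dynamic eye-close material instance and registers it as a zero-weight blendable on its PostProcess component.
; BlinkToClose, CloseToOpen and OpenToClose events play or reverse two timelines.
; Timeline updates feed SetEyeCloseLevel, which rewrites the blendable weight to animate the eyelid effect.
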(event Custom|SetEyeCloseLevel
  (params (Weight :type Float%20%28single-precision%29))
  (Utilities|Struct|SetmembersinWeightedBlendables (Utilities|Struct|BreakPostProcessSettings (Variables|/Script/Engine.PostProcessComponent|GetSettings (Variables|Default|GetPostProcess))) (Utilities|Array|MakeArray (Utilities|Struct|MakeWeightedBlendable Weight (Variables|Default|GetEyeEffMatInst)))))

(event Custom|BlinkToClose
  (bind _newtrack_0 (Timeline|TL_BlinkClose PlayFromStart)
    (:Update
      (CallFunction|SetEyeCloseLevel _newtrack_0))))

(event Custom|CloseToOpen
  (bind _newtrack_0 (Timeline|TL_Open PlayFromStart)
    (:Update
      (CallFunction|SetEyeCloseLevel _newtrack_0))))

(event Custom|OpenToClose
  (bind _newtrack_0 (Timeline|TL_Open ReverseFromEnd)
    (:Update
      (CallFunction|SetEyeCloseLevel _newtrack_0))))

(event EventBeginPlay)

(fn ConstructionScript
  (bind _returnvalue (Rendering|Material|CreateDynamicMaterialInstance "/Game/Blueprints/EyesEffect/ML_PE_EyeClose_Inst.ML_PE_EyeClose_Inst" "None" "None" :!class /Script/Engine.KismetMaterialLibrary))
  (bind _output_get (Variables|Default|SetEyeEffMatInst _returnvalue))
  (Variables|Default|SetSettings (Variables|/Script/Engine.PostProcessComponent|GetSettings (Variables|Default|GetPostProcess)))
  (Utilities|Struct|SetmembersinWeightedBlendables (Utilities|Struct|BreakPostProcessSettings (Variables|/Script/Engine.PostProcessComponent|GetSettings (Variables|Default|GetPostProcess))) (Utilities|Array|MakeArray (Utilities|Struct|MakeWeightedBlendable 0.0 _output_get))))