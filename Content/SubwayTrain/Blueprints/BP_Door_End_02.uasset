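; Subway train end door actor that the player opens with the E key.
; Overlapping Box enables input and opens a Gate, which lets E play a Timeline that slides the door mesh's relative location.
; Two further trigger volumes respond only to BP_ScrollingPlayer: one toggles a widget's visibility, the other a highlight overlay material on the door.
; Nothing closes the gate or disables input afterwards.
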(event OnComponentBeginOverlap(Box1)
  (params (OverlappedComponent :type Primitive%20Component%20Object%20Reference) (OtherActor :type Actor%20Object%20Reference) (OtherComp :type Primitive%20Component%20Object%20Reference) (OtherBodyIndex :type Integer) (bFromSweep :type Boolean) (SweepResult :type Hit%20Result%20Structure%20%28by%20ref%29))
  (Utilities|Casting|CastToBP_ScrollingPlayer OtherActor)
  (Rendering|SetVisibility (Variables|Default|GetWidget) true false))

(event OnComponentEndOverlap(Box1)
  (params (OverlappedComponent :type Primitive%20Component%20Object%20Reference) (OtherActor :type Actor%20Object%20Reference) (OtherComp :type Primitive%20Component%20Object%20Reference) (OtherBodyIndex :type Integer))
  (Utilities|Casting|CastToBP_ScrollingPlayer OtherActor)
  (Rendering|SetVisibility (Variables|Default|GetWidget) false false))

(event OnComponentBeginOverlap(Box2)
  (params (OverlappedComponent :type Primitive%20Component%20Object%20Reference) (OtherActor :type Actor%20Object%20Reference) (OtherComp :type Primitive%20Component%20Object%20Reference) (OtherBodyIndex :type Integer) (bFromSweep :type Boolean) (SweepResult :type Hit%20Result%20Structure%20%28by%20ref%29))
  (Utilities|Casting|CastToBP_ScrollingPlayer OtherActor)
  (Rendering|Material|SetOverlayMaterial (Variables|Default|Getendwall_door_01) "/Game/M_Highlight.M_Highlight" :!class /Script/Engine.MeshComponent))

(event OnComponentEndOverlap(Box2)
  (params (OverlappedComponent :type Primitive%20Component%20Object%20Reference) (OtherActor :type Actor%20Object%20Reference) (OtherComp :type Primitive%20Component%20Object%20Reference) (OtherBodyIndex :type Integer))
  (Utilities|Casting|CastToBP_ScrollingPlayer OtherActor)
  (Rendering|Material|SetOverlayMaterial (Variables|Default|Getendwall_door_01) 0 :!class /Script/Engine.MeshComponent))

(event OnComponentBeginOverlap(Box)
  (params (OverlappedComponent :type Primitive%20Component%20Object%20Reference) (OtherActor :type Actor%20Object%20Reference) (OtherComp :type Primitive%20Component%20Object%20Reference) (OtherBodyIndex :type Integer) (bFromSweep :type Boolean) (SweepResult :type Hit%20Result%20Structure%20%28by%20ref%29))
  (Input|EnableInput (Game|GetPlayerController 0))
  (Utilities|FlowControl|Gate true) ; enters at Open
)

(event Input|KeyboardEvents|E
  (params (Key :type Key%20Structure :default "None"))
  (:Pressed
    (Utilities|FlowControl|Gate true
      (:Exit
        (bind _新建轨道_0 (Timeline|时间轴 PlayFromStart)
          (:Update
            (Transformation|SetRelativeLocation (Variables|Default|Getendwall_door_01) (Math|Vector|MakeVector 0.0 _新建轨道_0 _新建轨道_0) false false)))))))

(fn ConstructionScript)