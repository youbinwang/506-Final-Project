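; Subway train end-wall door that the player swings open once by pressing E.
; Overlapping Box enables input and opens a gate, letting E play a timeline that drives the door's yaw, with PushOpen choosing the swing direction.
; Two further boxes toggle a prompt widget and a highlight overlay material for the scrolling character while interactable.
; Opening clears both cues and disables further interaction.
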(event OnComponentBeginOverlap(Box1)
  (params (OverlappedComponent :type Primitive%20Component%20Object%20Reference) (OtherActor :type Actor%20Object%20Reference) (OtherComp :type Primitive%20Component%20Object%20Reference) (OtherBodyIndex :type Integer) (bFromSweep :type Boolean) (SweepResult :type Hit%20Result%20Structure%20%28by%20ref%29))
  (Utilities|Casting|CastToBP_ScrollingCharacter OtherActor)
  (if (Variables|Default|GetIsInteractable)
    (Rendering|SetVisibility (Variables|Default|GetWidget) true false)))

(event OnComponentEndOverlap(Box1)
  (params (OverlappedComponent :type Primitive%20Component%20Object%20Reference) (OtherActor :type Actor%20Object%20Reference) (OtherComp :type Primitive%20Component%20Object%20Reference) (OtherBodyIndex :type Integer))
  (Utilities|Casting|CastToBP_ScrollingCharacter OtherActor)
  (Rendering|SetVisibility (Variables|Default|GetWidget) false false))

(event OnComponentBeginOverlap(Box2)
  (params (OverlappedComponent :type Primitive%20Component%20Object%20Reference) (OtherActor :type Actor%20Object%20Reference) (OtherComp :type Primitive%20Component%20Object%20Reference) (OtherBodyIndex :type Integer) (bFromSweep :type Boolean) (SweepResult :type Hit%20Result%20Structure%20%28by%20ref%29))
  (Utilities|Casting|CastToBP_ScrollingCharacter OtherActor)
  (if (Variables|Default|GetIsInteractable)
    (Rendering|Material|SetOverlayMaterial (Variables|Default|Getendwall_door_01) "/Game/Blueprints/Doors/M_Highlight.M_Highlight" :!class /Script/Engine.MeshComponent)))

(event OnComponentEndOverlap(Box2)
  (params (OverlappedComponent :type Primitive%20Component%20Object%20Reference) (OtherActor :type Actor%20Object%20Reference) (OtherComp :type Primitive%20Component%20Object%20Reference) (OtherBodyIndex :type Integer))
  (Utilities|Casting|CastToBP_ScrollingCharacter OtherActor)
  (Rendering|Material|SetOverlayMaterial (Variables|Default|Getendwall_door_01) 0 :!class /Script/Engine.MeshComponent))

(event OnComponentBeginOverlap(Box)
  (params (OverlappedComponent :type Primitive%20Component%20Object%20Reference) (OtherActor :type Actor%20Object%20Reference) (OtherComp :type Primitive%20Component%20Object%20Reference) (OtherBodyIndex :type Integer) (bFromSweep :type Boolean) (SweepResult :type Hit%20Result%20Structure%20%28by%20ref%29))
  (Input|EnableInput (Game|GetPlayerController 0))
  (Utilities|FlowControl|Gate true) ; enters at Open
)

(event Input|KeyboardEvents|E
  (params (Key :type Key%20Structure))
  (:Pressed
    (if (Variables|Default|GetIsInteractable)
      (Utilities|FlowControl|Gate true
        (:Exit
          (bind _dooropen (Timeline|时间轴 Play)
            (:Update
              (Transformation|SetRelativeRotation (Variables|Default|Getendwall_door_01) (Math|Rotator|MakeRotator 0.0 0.0 (Math|Float|SelectFloat (* _dooropen -1.0) _dooropen (Variables|Default|GetPushOpen))) false false)
              (Rendering|Material|SetOverlayMaterial (Variables|Default|Getendwall_door_01) 0 :!class /Script/Engine.MeshComponent)
              (Rendering|SetVisibility (Variables|Default|GetWidget) false false)
              (Variables|Default|SetIsInteractable false))))))))

(fn ConstructionScript)