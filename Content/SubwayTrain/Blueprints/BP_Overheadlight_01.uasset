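; BP_Overheadlight_01 is an overhead light for the subway train with a point light and a spot light.
; Its graphs hold two looping delay-based flicker sequences, an irregular flicker on both lights and a flash timed by FlashGap, but BeginPlay connects to neither.
; The construction script has setters for each light's intensity, color, attenuation, soft radius and temperature from variables, also left disconnected, so none of this logic runs.
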(event EventBeginPlay)

(fn ConstructionScript)