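; BP_LightController is a central controller that applies shared point and spot light settings to every BP_Overheadlight_01 in the level.
; Its Construction Script gathers those actors into AllLights and sets intensity, color, attenuation, soft source radius, visibility and temperature directly on their components from its own variables.
; The Event Graph does nothing at runtime, as its delay-based flashing loop is disconnected.
; Leftover unwired nodes in both graphs never execute.
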(event EventBeginPlay)

(event Collision|EventActorBeginOverlap
  (params (OtherActor :type Actor%20Object%20Reference)))

(event EventTick
  (params (DeltaSeconds :type Float%20%28single-precision%29)))

(fn ConstructionScript
  (bind _outactors (Actor|GetAllActorsOfClass "/Game/SubwayTrain/Blueprints/BP_Overheadlight_01.BP_Overheadlight_01_C"))
  (bind _output_get (Variables|Default|SetAllLights _outactors))
  (for _array_element _output_get
    (Rendering|Components|Light|SetIntensity (Variables|/Game/SubwayTrain/Blueprints/BP_Overheadlight_01.BP_Overheadlight_01_C|GetPointLight _array_element) (Variables|PointLight|GetPoints_Intensity))
    (Rendering|Components|Light|SetLightColor (Variables|/Game/SubwayTrain/Blueprints/BP_Overheadlight_01.BP_Overheadlight_01_C|GetPointLight _array_element) (Variables|PointLight|GetPoints_Color) true)
    (Rendering|Lighting|SetAttenuationRadius (Variables|/Game/SubwayTrain/Blueprints/BP_Overheadlight_01.BP_Overheadlight_01_C|GetPointLight _array_element) (Variables|PointLight|GetPoints_Attenuation))
    (Class|PointLightComponent|SetSoftSourceRadius (Variables|/Game/SubwayTrain/Blueprints/BP_Overheadlight_01.BP_Overheadlight_01_C|GetPointLight _array_element) (Variables|PointLight|GetPoints_SoftR))
    (Rendering|SetVisibility (Variables|/Game/SubwayTrain/Blueprints/BP_Overheadlight_01.BP_Overheadlight_01_C|GetPointLight _array_element) (Variables|PointLight|GetPoint_on/off) false)
    (Class|LightComponent|SetTemperature (Variables|/Game/SubwayTrain/Blueprints/BP_Overheadlight_01.BP_Overheadlight_01_C|GetPointLight _array_element) (Variables|PointLight|GetPoints_Temperature))
    (Rendering|Components|Light|SetIntensity (Variables|/Game/SubwayTrain/Blueprints/BP_Overheadlight_01.BP_Overheadlight_01_C|GetSpotLight _array_element) (Variables|Spot_Light|GetSpots_Brightness))
    (Rendering|Components|Light|SetLightColor (Variables|/Game/SubwayTrain/Blueprints/BP_Overheadlight_01.BP_Overheadlight_01_C|GetSpotLight _array_element) (Variables|Spot_Light|GetSpot%20Color) true)
    (Rendering|Lighting|SetAttenuationRadius (Variables|/Game/SubwayTrain/Blueprints/BP_Overheadlight_01.BP_Overheadlight_01_C|GetSpotLight _array_element) (Variables|Spot_Light|GetSpot%20Attenuation))
    (Class|PointLightComponent|SetSoftSourceRadius (Variables|/Game/SubwayTrain/Blueprints/BP_Overheadlight_01.BP_Overheadlight_01_C|GetSpotLight _array_element) (Variables|Spot_Light|GetSpot%20Soft%20R))
    (Rendering|SetVisibility (Variables|/Game/SubwayTrain/Blueprints/BP_Overheadlight_01.BP_Overheadlight_01_C|GetSpotLight _array_element) (Variables|Spot_Light|GetSpot_on/off) false)
    (Class|LightComponent|SetTemperature (Variables|/Game/SubwayTrain/Blueprints/BP_Overheadlight_01.BP_Overheadlight_01_C|GetSpotLight _array_element) (Variables|Spot_Light|GetSpot%20Temperature))))