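; Pistol skeletal mesh component that arms the scrolling character and makes its first shot trigger a level-wide lighting event.
; On BeginPlay it registers with its owner, snaps to the hand socket and adds the weapon input context.
; Each shoot input spawns a camera-aimed bullet with sound and muzzle flash.
; The first also kills all lights, then after a delay restores light controllers with new colors and cycle, and sets player walk speed.
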(event Input|EnhancedActionEvents|EnhancedInputActionIA_Shoot
  (params (ActionValue :type Boolean) (ElapsedSeconds :type Float%20%28double-precision%29) (TriggeredSeconds :type Float%20%28double-precision%29) (InputAction :type Input%20Action%20Object%20Reference :default "/Game/Weapon/FirstPerson/Input/Actions/IA_Shoot.IA_Shoot"))
  (bind _returnvalue (Game|GetPlayerCameraManager 0))
  (bind _returnvalue_2 (Transformation|GetSocketLocation "Ammo"))
  (bind _self self)
  (bind _projectileoffset (Variables|Default|GetProjectileOffset))
  (bind _returnvalue_3 (Transformation|GetSocketTransform _self "MuzzleFlash" "RTS_World"))
  (bind _returnvalue_4 (Camera|GetCameraRotation _returnvalue))
  (bind _returnvalue_5 (Math|Vector|RotateVector _projectileoffset _returnvalue_4))
  (bind _returnvalue_6 (+ _returnvalue_2 _returnvalue_5))
  (Utilities|FlowControl|Sequence
    (:then_0
      (Utilities|FlowControl|DoOnce false
        (:Completed
          (bind _outactors (Actor|GetAllActorsOfClass "/Game/Blueprints/Lights/BP_LightController.BP_LightController_C"))
          (bind _output_get (Variables|Default|SetOut%20Actors _outactors))
          (for _array_element _output_get
            (Variables|/Game/Blueprints/Lights/BP_LightController.BP_LightController_C|SetPoint_on/off _array_element false)
            (Variables|/Game/Blueprints/Lights/BP_LightController.BP_LightController_C|SetSpot_on/off _array_element false)
            (Default|Reset _array_element))
          (bind _outactors_2 (Actor|GetAllActorsOfClass "/Script/Engine.Light"))
          (for _array_element_2 _outactors_2
            (Rendering|SetVisibility (Variables|/Script/Engine.Light|GetLightComponent _array_element_2) false false))
          (Utilities|FlowControl|Delay 5.0)
          (for _array_element_3 (Variables|Default|GetOut%20Actors)
            (Variables|/Game/Blueprints/Lights/BP_LightController.BP_LightController_C|SetCycle _array_element_3 99.0)
            (Variables|/Game/Blueprints/Lights/BP_LightController.BP_LightController_C|SetPoints_Color _array_element_3 "(R=0.177888,G=0.219526,B=0.250158,A=1.000000)")
            (Variables|/Game/Blueprints/Lights/BP_LightController.BP_LightController_C|SetSpot%20Color _array_element_3 "(R=0.386430,G=0.396755,B=0.672443,A=1.000000)")
            (Variables|/Game/Blueprints/Lights/BP_LightController.BP_LightController_C|SetPoint_on/off _array_element_3 true)
            (Variables|/Game/Blueprints/Lights/BP_LightController.BP_LightController_C|SetSpot_on/off _array_element_3 true)
            (Default|Reset _array_element_3)
            (Variables|/Script/Engine.CharacterMovementComponent|SetMaxWalkSpeed (Variables|/Script/Engine.Character|GetCharacterMovement (Game|GetPlayerCharacter 0)) 1.2e+02)))))
    (:then_1
      ;[0.05 0.05 0.05] Fire - LM
      (Game|SpawnActorfromClass "/Game/Weapon/FirstPerson/Blueprints/BP_PistolBullet.BP_PistolBullet_C" (Math|Transform|MakeTransform _returnvalue_6 _returnvalue_4) "Undefined" "MultiplyWithRoot" 0 0)
      (Audio|PlaySoundatLocation "/Game/Weapon/FPWeapon/Audio/FirstPersonTemplateWeaponFire02.FirstPersonTemplateWeaponFire02" _returnvalue_6 "0, 0, 0" 1.0 1.0 0.0 0 0 0 0) ; Play firing sound
      (Effects|SpawnEmitterAttached "/Game/MilitaryWeapSilver/FX/P_Pistol_MuzzleFlash_01.P_Pistol_MuzzleFlash_01" _self "MuzzleFlash" (.location _returnvalue_3) (.rotation _returnvalue_3) "1.000000,1.000000,1.000000" "KeepWorldPosition"))))

(event EventBeginPlay
  ;[0.05098 0.05098 0.05098] Pistol Pick Up
  (bind _asbp_scrolling_character (Utilities|Casting|CastToBP_ScrollingCharacter (Components|GetOwner)))
  (bind _output_get (Variables|Default|SetScrollingCharacter _asbp_scrolling_character))
  (Variables|/Game/Framework/BP_ScrollingCharacter.BP_ScrollingCharacter_C|SetPistolWeapon _output_get self)
  (Transformation|AttachComponentToComponent (Variables|/Script/Engine.Character|GetMesh _output_get) "hand_r" "SnapToTarget" "SnapToTarget" "SnapToTarget" true)
  (Transformation|SetRelativeLocationAndRotation "-10.000000,2.500000,0.000000" "0.000000,100.000000,0.000000" false false)
  (Variables|/Game/Framework/BP_ScrollingCharacter.BP_ScrollingCharacter_C|SetHasPistol (Variables|Default|GetScrollingCharacter) true)
  ;;[0.05 0.05 0.05] Add Fire Input
  (bind _asbp_scrolling_player_controller (Utilities|Casting|CastToBP_ScrollingPlayerController (Pawn|GetController (Variables|Default|GetScrollingCharacter))))
  (Utilities|IsValid (PlayerController|LocalPlayerSubsystems|GetEnhancedInputLocalPlayerSubsystem _asbp_scrolling_player_controller)
    (:Is%20Valid
      (Input|AddMappingContext (PlayerController|LocalPlayerSubsystems|GetEnhancedInputLocalPlayerSubsystem _asbp_scrolling_player_controller) "/Game/Weapon/FirstPerson/Input/IMC_Weapons.IMC_Weapons" 1 "(bIgnoreAllPressedKeysUntilRelease=True,bForceImmediately=False,bNotifyUserSettings=False)"))))