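; Player controller that can hand a pawn over to a companion AI controller and take it back.
; BeginPlay spawns the PlayerRepresentationAIController; UseAI has it possess and start representing the pawn, while AIMoveTo and AILookAt forward target locations to it.
; StopAI repossesses the pawn and restores the view target.
; GetRepresentationAI spawns a replacement if the reference is invalid, but sets the reference to None instead of the new controller.
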(event Custom|UseAI
  (params (InPawn :type Pawn%20Object%20Reference))
  (bind _representationai (CallFunction|GetRepresentationAI))
  (Pawn|Possess _representationai InPawn)
  (Default|StartRepresentation _representationai))

(event Custom|AIMoveTo
  (params (TargetLoc :type Vector))
  (bind _representationai (CallFunction|GetRepresentationAI))
  (Default|SetTargetLoc _representationai TargetLoc))

(event Custom|AILookAt
  (params (InputPin :type Vector))
  (bind _representationai (CallFunction|GetRepresentationAI))
  (Default|SetLookLoc _representationai InputPin))

(event Custom|StopAI
  (params (InPawn :type Pawn%20Object%20Reference))
  (if (!= self (Pawn|GetController InPawn))
    (Pawn|Possess InPawn)
    (Game|Player|SetViewTargetwithBlend InPawn 0.0 "VTBlend_Linear" 0.0 false)))

(event EventBeginPlay
  (bind _self self)
  (bind _returnvalue (Game|SpawnActorfromClass "/Game/Blueprints/AI/PlayerRepresentationAIController.PlayerRepresentationAIController_C" (Transformation|GetActorTransform _self) "Undefined" "MultiplyWithRoot" 0 _self 0))
  (Variables|Default|SetRepresentationAI _returnvalue))

(fn ConstructionScript)

(fn GetRepresentationAI
  (bind _self self)
  (bind _returnvalue (Transformation|GetActorTransform _self))
  (Utilities|IsValid (Variables|Default|GetRepresentationAI)
    (:Is%20Valid
      _)
    (:Is%20Not%20Valid
      (Game|SpawnActorfromClass "/Game/Blueprints/AI/PlayerRepresentationAIController.PlayerRepresentationAIController_C" _returnvalue "Undefined" "MultiplyWithRoot" 0 _self 0)
      (Variables|Default|SetRepresentationAI 0)
      (Transformation|SetActorTransform (Components|GetOwner (Variables|Default|GetRepresentationAI)) _returnvalue)))
  (return (Variables|Default|GetRepresentationAI)))